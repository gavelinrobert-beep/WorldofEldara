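; BP_ConnectTest is a test actor that smoke-tests the Eldara client-server connection when play begins.
; It drives EldaraNetworkSubsystem through a hardcoded sequence: connect to localhost, log in as a test user, request the character list, create a character and select it.
; Fixed delays pace the requests instead of response callbacks, and a printed message announces world entry without checking any result.
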(event EventBeginPlay
  (bind _returnvalue (Subsystems|GetEldaraNetworkSubsystem))
  (Class|EldaraNetworkSubsystem|ConnecttoServer _returnvalue "127.0.0.1" 7777)
  (Class|EldaraNetworkSubsystem|SendLogin _returnvalue "TestUser")
  (Utilities|FlowControl|Delay 2.0)
  (Class|EldaraNetworkSubsystem|SendCharacterListRequest _returnvalue)
  (Utilities|FlowControl|Delay 2.0)
  (Class|EldaraNetworkSubsystem|SendCreateCharacter _returnvalue "Hero" "Sylvaen" "MemoryWarden" "Neutral" "None" (Utilities|Struct|MakeCharacterAppearance 1 1))
  (Utilities|FlowControl|Delay 0.2)
  (Class|EldaraNetworkSubsystem|SendSelectCharacter _returnvalue 1)
  (Development|PrintString "Entering world with character.."))

(event Collision|EventActorBeginOverlap
  (params (OtherActor :type Actor%20Object%20Reference)))

(event EventTick
  (params (DeltaSeconds :type Float%20%28single-precision%29)))

(fn ConstructionScript)